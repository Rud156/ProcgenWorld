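; DungeonGeneratorBP is the dungeon generator Blueprint, and its graph sets up the generator's on-screen UI.
; On BeginPlay it creates SeedDisplay and GenerateWorld widgets, stores them and adds both to the viewport.
; Each widget receives a reference back to the generator through its DungeonGenerator variable.
; The construction script is empty, and these graphs contain no generation logic.
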(event EventBeginPlay
  (Utilities|FlowControl|Sequence
    (:then_0
      (bind _returnvalue (UserInterface|CreateWidget "/Game/BluePrints/SeedDisplay.SeedDisplay_C"))
      (bind _output_get (Variables|Default|SetSeed%20Display _returnvalue))
      (UserInterface|Viewport|AddtoViewport _output_get 0)
      (Variables|/Game/BluePrints/SeedDisplay.SeedDisplay_C|SetDungeon%20Generator (Variables|Default|GetSeed%20Display) self))
    (:then_1
      (bind _returnvalue_2 (UserInterface|CreateWidget "/Game/BluePrints/GenerateWorld.GenerateWorld_C"))
      (bind _output_get_2 (Variables|Default|SetGenerate%20World _returnvalue_2))
      (UserInterface|Viewport|AddtoViewport _output_get_2 0)
      (Variables|/Game/BluePrints/GenerateWorld.GenerateWorld_C|SetDungeon%20Generator (Variables|Default|GetGenerate%20World) self))))

(fn ConstructionScript)