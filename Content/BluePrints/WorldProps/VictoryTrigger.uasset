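; VictoryTrigger is a world prop trigger that reacts to player overlap and manages a win screen widget.
; On BeginPlay it binds to the DungeonGenerator's generation-complete event, which removes and clears any existing win widget.
; The overlap event only casts to PlayerCharacter; the logic that creates and shows the WinDisplay widget is disconnected, so the win screen never appears from this trigger.
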(event Custom|Generation%20Complete
  (Utilities|IsValid (Variables|Default|GetWin%20Display%20Widget)
    (:Is%20Valid
      (Widget|RemovefromParent (Variables|Default|GetWin%20Display%20Widget))
      (Variables|Default|SetWin%20Display%20Widget 0))))

(event Collision|EventActorBeginOverlap
  (params (OtherActor :type Actor%20Object%20Reference))
  (Utilities|Casting|CastToPlayerCharacter OtherActor))

(event EventBeginPlay
  (bind _returnvalue (Actor|GetActorOfClass "/Script/ProcGenWorld.DungeonGenerator"))
  (EventDispatchers|BindEventtoOnGenerationComplete _returnvalue (delegate Custom|Generation%20Complete)))

(fn ConstructionScript)