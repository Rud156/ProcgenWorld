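; Player character Blueprint that clamps camera pitch at BeginPlay and binds handlers to player jump, land and move events.
; Jumping plays the jump section of JumpMontage on the player model, and a move event sends the character to the target location through AI MoveTo.
; The landed handler is empty, and the LandMontage section playback is left disconnected.
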(event Custom|Player%20Jumped
  (Animation|Montage|PlayMontage (Variables|Default|GetPlayerModel) "/Game/Animations/JumpMontage.JumpMontage" 1.0 0.0 "JumpMontage"))

(event Custom|Player%20Landed)

(event Custom|PLayer%20Moved
  (params (TargetLocation :type Vector))
  (AI|AIMoveTo self TargetLocation 0 5.0 false))

(event EventBeginPlay
  (bind _returnvalue (Game|GetPlayerCameraManager 0))
  (Utilities|FlowControl|Sequence
    (:then_0
      (Variables|/Script/Engine.PlayerCameraManager|SetViewPitchMin _returnvalue -2e+01)
      (Variables|/Script/Engine.PlayerCameraManager|SetViewPitchMax _returnvalue 5.0))
    (:then_1
      (EventDispatchers|BindEventtoOnPlayerJumped (delegate Custom|Player%20Jumped))
      (EventDispatchers|BindEventtoOnPlayerLanded (delegate Custom|Player%20Landed)))
    (:then_2
      (EventDispatchers|BindEventtoOnPlayerMoved (delegate Custom|PLayer%20Moved)))))

(fn ConstructionScript)