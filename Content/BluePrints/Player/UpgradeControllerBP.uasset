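; Upgrade controller Blueprint that shows and hides the player's upgrade display UI.
; On BeginPlay it creates an UpgradeDisplay widget for player 0, adds it to the viewport and keeps it hidden.
; DisplayUpgradesUI fills up to three slots from the first entries of an Upgrades map, setting name and description from the looked-up values, then reveals the widget.
; ClearUpgradesUI hides it again.
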(event EventBeginPlay
  (bind _returnvalue (UserInterface|CreateWidget "/Game/BluePrints/HUD/PlayerHUDDisplay/UpgradeDisplay.UpgradeDisplay_C" (Game|GetPlayerController 0)))
  (bind _output_get (Variables|Default|SetUpgrade%20Widget _returnvalue))
  (UserInterface|Viewport|AddtoViewport _output_get 0)
  (Widget|SetVisibility (Variables|Default|GetUpgrade%20Widget) "Hidden"))

(event EventDisplayUpgradesUI
  (params (upgrades :type Map%20of%20UpgradeType%20Enums%20to%20Strings :default "RestoreHP"))
  (bind _keys (Utilities|Map|Keys upgrades))
  (for (_array_element _array_index) _keys
    (if (< _array_index 3)
      (Default|SetUpgradeData (Variables|Default|GetUpgrade%20Widget) _array_index (.Value (Utilities|Map|Find upgrades _array_element)) (.Value (Utilities|Map|Find upgrades _array_element)))))
  (Widget|SetVisibility (Variables|Default|GetUpgrade%20Widget) "Visible"))

(event EventClearUpgradesUI
  (Widget|SetVisibility (Variables|Default|GetUpgrade%20Widget) "Hidden"))

(fn ConstructionScript)