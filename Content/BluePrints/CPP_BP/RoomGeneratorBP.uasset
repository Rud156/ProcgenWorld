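; RoomGeneratorBP is a room generator Blueprint that shows a RoomDisplay widget while the player is in its room.
; Each Tick it compares IsPlayerInRoom against the stored LastIsInRoom flag to detect entry and exit.
; On entry it creates the widget for player 0, adds it to the viewport and passes itself as RoomGenerator; on exit it removes the widget.
; The Blueprint itself contains no generation logic, and its construction script is empty.
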(event EventTick
  (params (DeltaSeconds :type Float%20%28single-precision%29))
  (Utilities|FlowControl|Sequence
    (:then_0
      (if (and (Class|RoomGenerator|IsPlayerinRoom) (not (Variables|Default|GetLast%20Is%20In%20Room)))
        (bind _returnvalue (UserInterface|CreateWidget "/Game/BluePrints/HUD/MiscDisplay/RoomDisplay.RoomDisplay_C" (Game|GetPlayerController 0)))
        (bind _output_get (Variables|Default|SetRoom%20Display _returnvalue))
        (UserInterface|Viewport|AddtoViewport _output_get 0)
        (Variables|/Game/BluePrints/HUD/MiscDisplay/RoomDisplay.RoomDisplay_C|SetRoom%20Generator (Variables|Default|GetRoom%20Display) self)))
    (:then_1
      (if (and (not (Class|RoomGenerator|IsPlayerinRoom)) (Variables|Default|GetLast%20Is%20In%20Room))
        (Utilities|IsValid (Variables|Default|GetRoom%20Display)
          (:Is%20Valid
            (Widget|RemovefromParent (Variables|Default|GetRoom%20Display))))))
    (:then_2
      (Variables|Default|SetLast%20Is%20In%20Room (Class|RoomGenerator|IsPlayerinRoom)))))

(fn ConstructionScript)